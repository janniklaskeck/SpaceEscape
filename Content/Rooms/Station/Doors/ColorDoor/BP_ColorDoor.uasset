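; BP_ColorDoor is a station door made of three parts that slide open separately.
; BeginPlay caches each part's starting relative location.
; The three open events each call their parent implementation, then play a timeline that offsets that part along its relative Y axis from the cached location.
; The Blueprint only animates the opening, with no closing logic or trigger conditions in its graphs.
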(event EventBeginPlay
  (|CallParentFunction)
  (Variables|Default|SetThirdInitialLocation (Variables|/Script/Engine.SceneComponent|GetRelativeLocation (Variables|Default|GetThirdDoorPart)))
  (Variables|Default|SetSecondInitialLocation (Variables|/Script/Engine.SceneComponent|GetRelativeLocation (Variables|Default|GetSecondDoorPart)))
  (Variables|Default|SetFirstInitialLocation (Variables|/Script/Engine.SceneComponent|GetRelativeLocation (Variables|Default|GetFirstDoorPart))))

(event EventOpenThirdPart
  (|CallParentFunction)
  (bind _progress (Timeline|ThirdPart Play)
    (:Update
      (Transformation|SetRelativeLocation (Variables|Default|GetThirdDoorPart) (+ (Variables|Default|GetThirdInitialLocation) (Math|Vector|MakeVector 0.0 _progress 0.0)) false false))))

(event EventOpenSecondPart
  (|CallParentFunction)
  (bind _progress (Timeline|SecondPart Play)
    (:Update
      (Transformation|SetRelativeLocation (Variables|Default|GetSecondDoorPart) (+ (Variables|Default|GetSecondInitialLocation) (Math|Vector|MakeVector 0.0 _progress 0.0)) false false))))

(event EventOpenFirstPart
  (|CallParentFunction)
  (bind _progress (Timeline|FirstPart Play)
    (:Update
      (Transformation|SetRelativeLocation (Variables|Default|GetFirstDoorPart) (+ (Variables|Default|GetFirstInitialLocation) (Math|Vector|MakeVector 0.0 _progress 0.0)) false false))))

(fn ConstructionScript)